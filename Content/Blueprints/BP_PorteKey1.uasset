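; BP_PorteKey1 is a door that the player can open and close with the T key while holding exactly two keys.
; Overlapping the Open component enables input if the player character's NbClef equals two; otherwise, or when overlap ends, input is disabled.
; A FlipFlop on T plays or reverses a timeline that rotates Door on roll and resets NbClef to zero on each update, consuming the keys.
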(event OnComponentBeginOverlap(Open)
  (params (OverlappedComponent :type Primitive%20Component%20Object%20Reference) (OtherActor :type Actor%20Object%20Reference) (OtherComp :type Primitive%20Component%20Object%20Reference) (OtherBodyIndex :type Integer) (bFromSweep :type Boolean) (SweepResult :type Hit%20Result%20Structure%20%28by%20ref%29))
  (bind _returnvalue (Game|GetPlayerController 0))
  (bind _asbp_player_character (Utilities|Casting|CastToBP_Player_Character (Game|GetPlayerCharacter 0)))
  (if (== (Variables|/Game/Blueprints/BP_Player_Character.BP_Player_Character_C|GetNbClef _asbp_player_character) 2)
    (Input|EnableInput _returnvalue)
    (else
      (Input|DisableInput _returnvalue))))

(event OnComponentEndOverlap(Open)
  (params (OverlappedComponent :type Primitive%20Component%20Object%20Reference) (OtherActor :type Actor%20Object%20Reference) (OtherComp :type Primitive%20Component%20Object%20Reference) (OtherBodyIndex :type Integer))
  (Input|DisableInput (Game|GetPlayerController 0)))

(event Input|KeyboardEvents|T
  (params (Key :type Key%20Structure))
  (:Pressed
    (Utilities|FlowControl|FlipFlop
      (:A
        (bind _rotation (Timeline|Timeline_0 Play)
          (:Update
            (Transformation|SetRelativeRotation (Variables|Default|GetDoor) (Math|Rotator|MakeRotator _rotation 0.0 0.0) false false)
            (bind _asbp_player_character (Utilities|Casting|CastToBP_Player_Character (Game|GetPlayerCharacter 0)))
            (Variables|/Game/Blueprints/BP_Player_Character.BP_Player_Character_C|SetNbClef _asbp_player_character 0))))
      (:B
        (Timeline|Timeline_0 Reverse)))))

(fn ConstructionScript)