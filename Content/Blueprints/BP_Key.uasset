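; BP_Key is a collectible key actor that adds to the player's key count when picked up.
; Tick turns its point light off every frame, and the VoirClef event lights it up, so it glows only while that event keeps firing.
; RamasserClef casts the player pawn to BP_Player_Character, increments NbClef and destroys the key.
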(event Custom|VoirClef
  (Rendering|Components|Light|SetIntensity (Variables|Default|GetPointLight) 8e+01))

(event Custom|RamasserClef
  (bind _asbp_player_character (Utilities|Casting|CastToBP_Player_Character (Game|GetPlayerCharacter 0)))
  (bind _result (Math|Integer|IncrementInt (Variables|/Game/Blueprints/BP_Player_Character.BP_Player_Character_C|GetNbClef _asbp_player_character))
    (:%20%20
      (Variables|/Game/Blueprints/BP_Player_Character.BP_Player_Character_C|SetNbClef _asbp_player_character _result)
      (Actor|DestroyActor))))

(event EventTick
  (params (DeltaSeconds :type Float%20%28single-precision%29))
  (Rendering|Components|Light|SetIntensity (Variables|Default|GetPointLight) 0.0))

(event Input|KeyboardEvents|E
  (params (Key :type Key%20Structure)))

(fn ConstructionScript)