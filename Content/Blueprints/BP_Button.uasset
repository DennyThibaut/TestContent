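; BP_Button is a pushable button that lights up on demand and counts presses on the player character.
; Tick resets its PointLight to zero every frame, so the glow from VoirButton ("see button") lasts only while that event keeps being called.
; PushButton casts the player to BP_Player_Character and increments its ButtonPushed counter, with no guard against repeat presses.
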(event Custom|VoirButton
  (Rendering|Components|Light|SetIntensity (Variables|Default|GetPointLight) 8e+01))

(event Custom|PushButton
  (bind _asbp_player_character (Utilities|Casting|CastToBP_Player_Character (Game|GetPlayerCharacter 0)))
  (bind _result (Math|Integer|IncrementInt (Variables|/Game/Blueprints/BP_Player_Character.BP_Player_Character_C|GetButtonPushed? _asbp_player_character))
    (:%20%20
      (Variables|/Game/Blueprints/BP_Player_Character.BP_Player_Character_C|SetButtonPushed? _asbp_player_character _result))))

(event EventTick
  (params (DeltaSeconds :type Float%20%28single-precision%29))
  (Rendering|Components|Light|SetIntensity (Variables|Default|GetPointLight) 0.0))

(fn ConstructionScript)